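; BP_PlayerController is a player controller that sets up UI and input mode when play begins, based on the current level.
; In levels whose name contains "mainmenu", it creates and stores the WBP_MainMenu widget, adds it to the viewport, shows the cursor and focuses UI-only input on the menu.
; In all other levels it hides the cursor and switches to game-only input.
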(event EventBeginPlay
  ;[0 0.4 1] Sets up UI
  (bind _returnvalue (Game|GetCurrentLevelName true))
  (if (Utilities|String|Contains _returnvalue "mainmenu")
    (Variables|Default|SetbShowMouseCursor true)
    (bind _returnvalue_2 (UserInterface|CreateWidget "/Game/Blueprints/MainMenu/WBP_MainMenu.WBP_MainMenu_C"))
    (bind _output_get (Variables|Default|SetMainMenuWidget _returnvalue_2))
    (UserInterface|Viewport|AddtoViewport _output_get 0)
    (Input|SetInputModeUIOnly self _output_get "DoNotLock")
    (else
      (Variables|Default|SetbShowMouseCursor false)
      (Input|SetInputModeGameOnly self))))

(fn ConstructionScript)